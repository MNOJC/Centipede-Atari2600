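; Grid actor that defines a SizeX by SizeY grid on the world YZ plane at X=0, starting at the origin.
; Tick redraws a four-segment debug circle at each point, spaced by CellSize, with SizeX running along Z and SizeY along Y.
; Helper functions return the grid center and bounds; the max bound uses SizeY-1 on Y but full SizeX on Z.
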(event EventBeginPlay)

(event Collision|EventActorBeginOverlap
  (params (OtherActor :type Actor%20Object%20Reference)))

(event EventTick
  (params (DeltaSeconds :type Float%20%28single-precision%29))
  (for _index (range 0 (- (Variables|Default|GetSizeX) 1))
    (for _index_2 (range 0 (- (Variables|Default|GetSizeY) 1))
      (Rendering|Debug|DrawDebugCircle (Math|Vector|MakeVector 0.0 (* (Math|Conversions|ToFloat(Integer) _index_2) (Variables|Default|GetCellSize)) (* (Math|Conversions|ToFloat(Integer) _index) (Variables|Default|GetCellSize))) 3.0 4 "(R=1.000000,G=0.879387,B=0.000000,A=1.000000)" 0.0 2.0 "0.000000,1.000000,0.000000" "0.000000,0.000000,1.000000"))))

(fn ConstructionScript)

(fn GetGridCenterLocation
  (bind _cellsize (Variables|Default|GetCellSize))
  (return (Math|Vector|MakeVector 0.0 (* (/ (Math|Conversions|ToFloat(Integer) (Variables|Default|GetSizeY)) 2.0) _cellsize) (* (/ (Math|Conversions|ToFloat(Integer) (Variables|Default|GetSizeX)) 2.0) _cellsize))))

(fn GetGridBounds
  (bind _cellsize (Variables|Default|GetCellSize))
  (return (Math|Vector|MakeVector 0.0 (* (Math|Conversions|ToFloat(Integer) (- (Variables|Default|GetSizeY) 1)) _cellsize) (* (Math|Conversions|ToFloat(Integer) (Variables|Default|GetSizeX)) _cellsize)) "0, 0, 0"))