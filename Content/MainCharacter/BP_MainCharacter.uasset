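; BP_MainCharacter is the player character, which moves along the world Y axis and fires magic wand projectiles.
; On possession it adds the default Enhanced Input mapping context, and movement input drives the sideways motion.
; On BeginPlay it switches the view to the game camera actor and caches the grid generator, whose bounds clamp its Y position every Tick.
; The shoot input spawns a BP_MagicWandProjectile at the character's location.
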(event Input|EnhancedActionEvents|EnhancedInputActionIA_Movement
  (params (ActionValue :type Vector%202D%20Structure) (ElapsedSeconds :type Float%20%28double-precision%29) (TriggeredSeconds :type Float%20%28double-precision%29) (InputAction :type Input%20Action%20Object%20Reference :default "/Game/Input/InputActions/IA_Movement.IA_Movement"))
  (Pawn|Input|AddMovementInput "0.000000,1.000000,0.000000" (.x ActionValue) true))

(event Input|EnhancedActionEvents|EnhancedInputActionIA_Shoot
  (params (ActionValue :type Boolean) (ElapsedSeconds :type Float%20%28double-precision%29) (TriggeredSeconds :type Float%20%28double-precision%29) (InputAction :type Input%20Action%20Object%20Reference :default "/Game/Input/InputActions/IA_Shoot.IA_Shoot"))
  (:Started
    (Game|SpawnActorfromClass "/Game/MainCharacter/BP_MagicWandProjectile.BP_MagicWandProjectile_C" (Math|Transform|MakeTransform (Transformation|GetActorLocation) "0, 0, 0" "1.000000,1.000000,1.000000") "AlwaysSpawn" "MultiplyWithRoot" 0 0)))

(event Collision|EventActorBeginOverlap
  (params (OtherActor :type Actor%20Object%20Reference)))

(event EventTick
  (params (DeltaSeconds :type Float%20%28single-precision%29))
  (bind _returnvalue (Transformation|GetActorLocation))
  (bind _gridgenerator (Variables|Default|GetGridGenerator))
  (bind (_maxbounds _minbounds) (Default|GetGridBounds _gridgenerator))
  (Transformation|SetActorLocation (Math|Vector|MakeVector (.x _returnvalue) (Math|Float|Clamp(Float) (.y _returnvalue) (.y _minbounds) (.y _maxbounds)) (.z _returnvalue)) false false))

(event EventPossessed
  (params (NewController :type Controller%20Object%20Reference))
  (bind _aspc_main_character (Utilities|Casting|CastToPC_MainCharacter NewController))
  (Input|AddMappingContext (PlayerController|LocalPlayerSubsystems|GetEnhancedInputLocalPlayerSubsystem _aspc_main_character) "/Game/Input/IMC_Default.IMC_Default" 0 "(bIgnoreAllPressedKeysUntilRelease=True,bForceImmediately=False,bNotifyUserSettings=False)"))

(event EventBeginPlay
  (bind _returnvalue (Actor|GetActorOfClass "/Game/Camera/BP_GameCamera.BP_GameCamera_C"))
  (Game|Player|SetViewTargetwithBlend (Game|GetPlayerController 0) _returnvalue 0.0 "VTBlend_Linear" 0.0 false)
  (bind _returnvalue_2 (Actor|GetActorOfClass "/Game/Grid/BP_GridGenerator.BP_GridGenerator_C"))
  (Variables|Default|SetGridGenerator _returnvalue_2))

(fn ConstructionScript)